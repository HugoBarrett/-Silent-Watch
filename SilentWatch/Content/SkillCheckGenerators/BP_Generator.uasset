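; BP_Generator is an interactable generator that puts the player into a skill check.
; Tick polls the top-down character and, while it is interacting with this actor, calls StartGenerator, which creates WBP_SkillCheck and locks movement and look input.
; EndGenerator, not called here, removes the widget, restores control and destroys the generator.
; Two construction-sized spheres swap outer and inner prompt icons by player proximity; Interact only returns false.
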(event OnComponentBeginOverlap(InnerSphereCollision)
  (params (OverlappedComponent :type Primitive%20Component%20Object%20Reference) (OtherActor :type Actor%20Object%20Reference) (OtherComp :type Primitive%20Component%20Object%20Reference) (OtherBodyIndex :type Integer) (bFromSweep :type Boolean) (SweepResult :type Hit%20Result%20Structure%20%28by%20ref%29))
  ;[0.15 0.15 0.15 0.5] Inner Sphere
  (if (== OtherActor (Game|GetPlayerCharacter 0))
    (Rendering|SetVisibility (Variables|Default|GetInnerInteractIcon) true false)
    (Rendering|SetVisibility (Variables|Default|GetOuterInteractIcon) false false)))

(event OnComponentEndOverlap(InnerSphereCollision)
  (params (OverlappedComponent :type Primitive%20Component%20Object%20Reference) (OtherActor :type Actor%20Object%20Reference) (OtherComp :type Primitive%20Component%20Object%20Reference) (OtherBodyIndex :type Integer))
  ;[0.15 0.15 0.15 0.5] Inner Sphere
  (if (== (Game|GetPlayerCharacter 0) OtherActor)
    (Rendering|SetVisibility (Variables|Default|GetInnerInteractIcon) false false)
    (Rendering|SetVisibility (Variables|Default|GetOuterInteractIcon) true false)))

(event OnComponentBeginOverlap(OuterSphereCollision)
  (params (OverlappedComponent :type Primitive%20Component%20Object%20Reference) (OtherActor :type Actor%20Object%20Reference) (OtherComp :type Primitive%20Component%20Object%20Reference) (OtherBodyIndex :type Integer) (bFromSweep :type Boolean) (SweepResult :type Hit%20Result%20Structure%20%28by%20ref%29))
  ;[0.15 0.15 0.15 0.5] Outer Sphere
  (if (== OtherActor (Game|GetPlayerCharacter 0))
    (Rendering|SetVisibility (Variables|Default|GetOuterInteractIcon) true false)))

(event OnComponentEndOverlap(OuterSphereCollision)
  (params (OverlappedComponent :type Primitive%20Component%20Object%20Reference) (OtherActor :type Actor%20Object%20Reference) (OtherComp :type Primitive%20Component%20Object%20Reference) (OtherBodyIndex :type Integer))
  ;[0.15 0.15 0.15 0.5] Outer Sphere
  (if (== (Game|GetPlayerCharacter 0) OtherActor)
    (Rendering|SetVisibility (Variables|Default|GetOuterInteractIcon) false false)))

(event Custom|End%20Generator
  (bind _returnvalue (Game|GetPlayerController 0))
  ;[0.15 0.15 0.15 0.5] End Generator
  (Utilities|FlowControl|Sequence
    (:then_0
      (bind _skillcheckref (Variables|Default|GetSkillCheckRef)
        (:then
          (Widget|RemovefromParent _skillcheckref)
          (Variables|Default|SetSkillCheckRef 0)
          (Actor|DestroyActor))
        (:else)))
    (:then_1
      (Input|ResetIgnoreLookInput _returnvalue)
      (Variables|/Script/Engine.PlayerController|SetbShowMouseCursor _returnvalue false)
      (Input|SetInputModeGameOnly _returnvalue false)
      (Pawn|Components|CharacterMovement|SetMovementMode (Variables|/Script/Engine.Character|GetCharacterMovement (Game|GetPlayerCharacter 0)) "MOVE_Walking" 0))))

(event Custom|Start%20Generator
  (bind _returnvalue (Game|GetPlayerController 0))
  ;[0.15 0.15 0.15 0.5] Start Generator
  (bind _returnvalue_2 (UserInterface|CreateWidget "/Game/SkillCheckGenerators/WBP_SkillCheck.WBP_SkillCheck_C"))
  (bind _output_get (Variables|Default|SetSkillCheckRef _returnvalue_2))
  (UserInterface|Viewport|AddtoViewport _output_get 0)
  (Input|SetIgnoreLookInput _returnvalue true)
  (Variables|/Script/Engine.PlayerController|SetbShowMouseCursor _returnvalue false)
  (Input|SetInputModeGameandUI _returnvalue 0 "DoNotLock" true false)
  (Pawn|Components|CharacterMovement|DisableMovement (Variables|/Script/Engine.Character|GetCharacterMovement (Game|GetPlayerCharacter 0))))

(event Custom|Destroy
  (Development|PrintString "worked")
  (Utilities|FlowControl|Delay 0.5)
  (Actor|DestroyActor))

(event EventBeginPlay
  (bind _asbp_top_down_character (Utilities|Casting|CastToBP_TopDownCharacter (Game|GetPlayerCharacter 0)))
  (Variables|Default|SetCharacterRef _asbp_top_down_character))

(event EventTick
  (params (DeltaSeconds :type Float%20%28single-precision%29))
  (bind _characterref (Variables|Default|GetCharacterRef))
  (if (and (Variables|/Game/TopDown/Blueprints/BP_TopDownCharacter.BP_TopDownCharacter_C|GetIs%20Interacting? _characterref) (== (Variables|/Game/TopDown/Blueprints/BP_TopDownCharacter.BP_TopDownCharacter_C|GetHit%20Actor _characterref) self))
    (CallFunction|StartGenerator)))

(fn ConstructionScript
  (Components|Sphere|SetSphereRadius (Variables|Default|GetInnerSphereCollision) (Variables|Public|GetInnerSphereRadius) true)
  (Components|Sphere|SetSphereRadius (Variables|Default|GetOuterSphereCollision) (Variables|Public|GetOuterSphereRadius) true))

(fn Interact
  (params (Character :type Character%20Object%20Reference))
  (return false))