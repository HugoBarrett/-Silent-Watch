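; Enemy character that advances on the lighthouse and switches to chasing and attacking the player once it sees them.
; Until then, Tick repeatedly issues AI moves to the lighthouse focus point actor.
; Pawn sensing sets a seeing flag and triggers a move to player 0, stopping within a configurable radius.
; On arrival it plays an attack montage, using its length as a delay before re-enabling attacks.
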(event OnSeePawn(PawnSensing)
  (params (Pawn :type Pawn%20Object%20Reference))
  (Variables|Default|SetIsSeeingPlayer true)
  (CallFunction|FollowPlayer))

(event Custom|FollowPlayer
  (Variables|Default|SetCanAttack true)
  (if (Variables|Default|GetIsSeeingPlayer)
    (AI|AIMoveTo self "0, 0, 0" (Game|GetPlayerCharacter 0) (Variables|Default|GetAreaThatTheEnemyWillStopAt) false
      (:OnSuccess
        (if (Variables|Default|GetCanAttack)
          (Variables|Default|SetCanAttack false)
          (bind _returnvalue (Animation|PlayAnimMontage "/Game/Characters/Mannequins/Anims/Unarmed/Attack/MM_Attack_01_Montage.MM_Attack_01_Montage" 1.0 "None"))
          (Utilities|FlowControl|Delay _returnvalue)
          (Variables|Default|SetCanAttack true))))
    (else
      (Variables|Default|SetIsSeeingPlayer false))))

(event Custom|MoveTowardsLightHouse
  (bind _returnvalue (Actor|GetActorOfClass "/Game/AI/Bp_LighthouseAiFocusPoint.Bp_LighthouseAiFocusPoint_C"))
  (AI|AIMoveTo self (Transformation|GetActorLocation _returnvalue) 0 5.0 false))

(event Collision|EventActorBeginOverlap
  (params (OtherActor :type Actor%20Object%20Reference)))

(event EventTick
  (params (DeltaSeconds :type Float%20%28single-precision%29))
  (if (not (Variables|Default|GetIsSeeingPlayer))
    (CallFunction|MoveTowardsLightHouse)))

(fn ConstructionScript)