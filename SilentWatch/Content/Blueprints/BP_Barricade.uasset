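; BP_Barricade is a placeable barricade that follows the top-down character while held and stays put once placed.
; On BeginPlay it attaches to the character's Positioner and shows a placing material.
; While a gate is open, each Tick traces downward and moves the Barricade component to the ground hit point.
; Placed detaches it, applies the gray grid material and closes the gate to end the snapping.
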(event Custom|Placed
  ;[0.15 0.15 0.15 0.5] Place me B
  (Transformation|DetachFromActor "KeepWorld" "KeepWorld" "KeepWorld")
  (Rendering|Material|SetMaterial (Variables|Default|GetBarricade) 0 "/Game/LevelPrototyping/Materials/MI_PrototypeGrid_Gray.MI_PrototypeGrid_Gray")
  ;[0.15 0.15 0.15 0.5] Snap to ground B
  (Utilities|FlowControl|Gate false) ; enters at Close
)

(event EventBeginPlay
  ;[0.15 0.15 0.15 0.5] Follow player while held B
  (bind _returnvalue (Actor|GetActorOfClass "/Game/TopDown/Blueprints/BP_TopDownCharacter.BP_TopDownCharacter_C"))
  (Transformation|AttachComponentToComponent (Variables|/Game/TopDown/Blueprints/BP_TopDownCharacter.BP_TopDownCharacter_C|GetPositioner _returnvalue) "None" "KeepWorld" "KeepWorld" "KeepWorld" true)
  (Rendering|Material|SetMaterial (Variables|Default|GetBarricade) 0 "/Game/Materials/M_BarricadePlacing.M_BarricadePlacing"))

(event EventTick
  (params (DeltaSeconds :type Float%20%28single-precision%29))
  ;[0.15 0.15 0.15 0.5] Snap to ground B
  (Utilities|FlowControl|Gate false
    (:Exit
      (bind _outhit (Collision|LineTraceByChannel (Transformation|GetActorLocation) (+ (Transformation|GetActorLocation) "0.000000,0.000000,-1000.000000") "TraceTypeQuery3" false 0 "None"))
      (Transformation|SetWorldLocation (Variables|Default|GetBarricade) (.ImpactPoint (Collision|BreakHitResult _outhit)) false false))))

(fn ConstructionScript)