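; Day/night cycle actor that rotates a directional light as the sun and counts days.
; It starts in daytime, then a timeline adds a fixed, frame-rate-dependent pitch step on each update.
; Exact float checks at 360 and 180 degrees trigger NightStart or DayStart on BP_TopDownCharacter, wrapping rotation at night and incrementing DayCount at day.
; Debug prints show rotation, phase and day count.
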(event EventBeginPlay
  ;[0.15 0.15 0.15 0.5] Day/Night cycle B
  (Variables|Default|SetSunRotation 1.8e+02)
  (Variables|Default|SetDayCount 1)
  (bind _returnvalue (Actor|GetActorOfClass "/Game/TopDown/Blueprints/BP_TopDownCharacter.BP_TopDownCharacter_C"))
  (Default|DayStart _returnvalue)
  (Timeline|SunCycle Play
    (:Update
      (Variables|Default|SetSunRotation (+ (Variables|Default|GetSunRotation) 0.05))
      (Development|PrintString (Utilities|String|ToString(Float) (Variables|Default|GetSunRotation)))
      (if (== 3.6e+02 (Variables|Default|GetSunRotation))
        (Development|PrintString "Night")
        (Variables|Default|SetSunRotation 0.0)
        (bind _returnvalue_2 (Actor|GetActorOfClass "/Game/TopDown/Blueprints/BP_TopDownCharacter.BP_TopDownCharacter_C"))
        (Default|NightStart _returnvalue_2)
        (elif (== 1.8e+02 (Variables|Default|GetSunRotation))
          (Development|PrintString "Day")
          (bind _returnvalue_3 (Actor|GetActorOfClass "/Game/TopDown/Blueprints/BP_TopDownCharacter.BP_TopDownCharacter_C"))
          (Default|DayStart _returnvalue_3)
          (bind _output_get (Variables|Default|SetDayCount (+ (Variables|Default|GetDayCount) 1)))
          (Development|PrintString (Utilities|String|ToString(Integer) _output_get))))
      (Transformation|SetRelativeRotation (Variables|Default|GetDirectionalLight) (Math|Rotator|MakeRotator 0.0 (Variables|Default|GetSunRotation) 0.0) false false))))

(fn ConstructionScript)