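; Potion shop actor that opens a store menu when the top-down player character overlaps its trigger.
; Overlap freezes movement, swaps to the shop input context, and plays the start audio from the store's DT_PotionStores row.
; When that audio finishes, it creates WBP_PotionStore with the row data.
; End plays the exit audio, restores movement and input, and clears references; sounds are async-loaded and weight-gated.
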(event OnComponentBeginOverlap(Trigger)
  (params (OverlappedComponent :type Primitive%20Component%20Object%20Reference) (OtherActor :type Actor%20Object%20Reference) (OtherComp :type Primitive%20Component%20Object%20Reference) (OtherBodyIndex :type Integer) (bFromSweep :type Boolean) (SweepResult :type Hit%20Result%20Structure%20%28by%20ref%29))
  ;[0.15 0.1343 0.03028 0.5] Cache player
  (bind _asbp_top_down_character (Utilities|Casting|CastToBP_TopDownCharacter OtherActor))
  (Variables|Default|SetPlayer%20Character%20Ref _asbp_top_down_character)
  (Variables|Default|SetPlayer%20Controller (Game|GetPlayerController 0))
  (CallFunction|DisablePlayer)
  (bind _returnvalue (Utilities|GetDataTableRow "/Game/Shop/Food/Stores/DT_PotionStores.DT_PotionStores" (Variables|Default|GetStores%20Row%20Name))
    (:then
      (EventDispatchers|AssignOnAudioFinished (Variables|Default|GetAudio) (delegate Custom|OnAudioFinished_Event))
      (CallFunction|PlayAudioAsync (.StartAudio (Utilities|Struct|BreakS_PotionStore _returnvalue)) 1))
    (:RowNotFound
      (Development|PrintString "Error: Store Name Not Found"))))

(event Custom|Play%20Audio%20Async
  (params (Audio :type Sound%20Cue%20Soft%20Object%20Reference) (Weight :type Integer))
  ;[0.03501 0.03272 0.15 0.5] Play Audio Async With A Weight
  (if (and (not (Audio|Components|Audio|IsPlaying (Variables|Default|GetAudio))) (Math|Random|RandomBoolwithWeight (Math|Conversions|ToFloat(Integer) Weight)))
    (bind _object (Utilities|AsyncLoadAsset Audio)
      (:Completed
        (bind _assound_cue (Utilities|Casting|CastToSoundCue _object))
        (Audio|Components|Audio|SetSound (Variables|Default|GetAudio) _assound_cue)
        (Audio|Components|Audio|Play (Variables|Default|GetAudio) 0.0)))))

(event Custom|OnAudioFinished_Event
  (EventDispatchers|UnbindEventfromOnAudioFinished (Variables|Default|GetAudio) (delegate Custom|OnAudioFinished_Event))
  (CallFunction|SetupUI (stale OnComponentBeginOverlap(Trigger) _returnvalue)))

(event Custom|End
  (bind _returnvalue (Utilities|GetDataTableRow "/Game/Shop/Food/Stores/DT_PotionStores.DT_PotionStores" (Variables|Default|GetStores%20Row%20Name))
    (:then
      (CallFunction|PlayAudioAsync (.ExitAudio (Utilities|Struct|BreakS_PotionStore _returnvalue)) 1)
      (CallFunction|EnablePlayer)
      ;[0.15 0.0103 0.01746 0.5] Remove Variables
      (Variables|/Game/TopDown/Blueprints/BP_TopDownCharacter.BP_TopDownCharacter_C|SetCurrent%20Shop%20Menu (Variables|Default|GetPlayer%20Character%20Ref) 0)
      (Variables|Default|SetPlayer%20Character%20Ref 0)
      (Variables|Default|SetPlayer%20Controller 0))))

(fn ConstructionScript)

(fn DisablePlayer
  (bind _player_character_ref (Variables|Default|GetPlayer%20Character%20Ref))
  (bind _player_controller (Variables|Default|GetPlayer%20Controller))
  (bind _returnvalue (PlayerController|LocalPlayerSubsystems|GetEnhancedInputLocalPlayerSubsystem _player_controller))
  (bind _charactermovement (Variables|/Script/Engine.Character|GetCharacterMovement _player_character_ref))
  ;[0.15 0.03592 0.03449 0.5] Disable Movement
  (Pawn|Components|CharacterMovement|SetMovementMode _charactermovement "MOVE_None" 0)
  (Components|Movement|StopMovementImmediately _charactermovement)
  (Variables|/Script/Engine.PlayerController|SetbShowMouseCursor (Variables|Default|GetPlayer%20Controller) true)
  ;[0.15 0.1297 0.01997 0.5] Switch Player Imput
  (Input|RemoveMappingContext _returnvalue "/Game/TopDown/Input/IMC_TopDown.IMC_TopDown" "(bIgnoreAllPressedKeysUntilRelease=True,bForceImmediately=False,bNotifyUserSettings=False)")
  (Input|AddMappingContext _returnvalue "/Game/Shop/InputMapping/IMC_Shop.IMC_Shop" 0 "(bIgnoreAllPressedKeysUntilRelease=True,bForceImmediately=False,bNotifyUserSettings=False)"))

(fn EnablePlayer
  (bind _player_controller (Variables|Default|GetPlayer%20Controller))
  (bind _returnvalue (PlayerController|LocalPlayerSubsystems|GetEnhancedInputLocalPlayerSubsystem _player_controller))
  ;[0.02542 0.15 0.0165 0.5] Enable Movement
  (Pawn|Components|CharacterMovement|SetMovementMode (Variables|/Script/Engine.Character|GetCharacterMovement (Variables|Default|GetPlayer%20Character%20Ref)) "MOVE_Walking" 0)
  (Variables|/Script/Engine.PlayerController|SetbShowMouseCursor (Variables|Default|GetPlayer%20Controller) true)
  ;[0.15 0.1297 0.01997 0.5] Switch Player Imput
  (Input|RemoveMappingContext _returnvalue "/Game/Shop/InputMapping/IMC_Shop.IMC_Shop" "(bIgnoreAllPressedKeysUntilRelease=True,bForceImmediately=False,bNotifyUserSettings=False)")
  (Input|AddMappingContext _returnvalue "/Game/TopDown/Input/IMC_TopDown.IMC_TopDown" 0 "(bIgnoreAllPressedKeysUntilRelease=True,bForceImmediately=False,bNotifyUserSettings=False)"))

(fn SetupUI
  (params (StoreInfo :type S%20Potion%20Store%20Structure))
  (bind _returnvalue (UserInterface|CreateWidget "/Game/Shop/WBP_PotionStore.WBP_PotionStore_C" (Variables|Default|GetPlayer%20Controller) self StoreInfo))
  (Variables|/Game/TopDown/Blueprints/BP_TopDownCharacter.BP_TopDownCharacter_C|SetCurrent%20Shop%20Menu (Variables|Default|GetPlayer%20Character%20Ref) _returnvalue)
  (UserInterface|Viewport|AddtoViewport _returnvalue 0)
  (Input|SetInputModeGameandUI (Variables|Default|GetPlayer%20Controller) _returnvalue "DoNotLock" true false))